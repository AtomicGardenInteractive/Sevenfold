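; BP_Cain_ABEL_ONE is a possessable Abel actor that keeps an invisible platform beneath it while unpossessed.
; It spawns an owned BP_InvisPlatform on BeginPlay and a second after unpossession.
; Possession waits briefly, then destroys its owned platforms; both transitions jump the Locomotion animation state machine to matching nodes.
; AnyDamage is empty, leaving the corpse-and-platform spawn logic intended for spike deaths disconnected.
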(event EventBeginPlay
  ;[1 1 1] Spawn make platform
  (Game|SpawnActorfromClass "/Game/BluePrints/Cain/Cain_Possesed/BP_InvisPlatform.BP_InvisPlatform_C" (Math|Conversions|ToTransform(Vector) (Math|Transform|TransformLocation (Transformation|GetActorTransform self) "0, 0,-90.000000")) "AlwaysSpawn" self 0))

(event Collision|EventActorBeginOverlap
  (params (OtherActor :type Actor%20Object%20Reference)))

(event EventTick
  (params (DeltaSeconds :type Float%20%28single-precision%29))
  (|CallParentFunction DeltaSeconds) ; This node is disabled and will not be called.\nDrag off pins to build functionality.
)

(event EventPossessed
  (params (NewController :type Controller%20Object%20Reference))
  ;[1 1 1] When Possessing animate and destory the plaform
  (Utilities|FlowControl|Delay 0.2)
  (Class|PaperZDAnimInstance|JumptoNode (Variables|/Script/PaperZD.PaperZDAnimationComponent|GetAnimInstance (Variables|Default|GetAnimationComponent)) "Possessed" "Locomotion")
  (bind _outactors (Actor|GetAllActorsOfClass "/Game/BluePrints/Cain/Cain_Possesed/BP_InvisPlatform.BP_InvisPlatform_C"))
  (bind _array_element (Utilities|Array|ForEachLoopwithBreak _outactors)
    (:LoopBody
      (if (== self (Components|GetOwner _array_element))
        (Actor|DestroyActor _array_element)))))

(event EventUnpossessed
  (params (OldController :type Controller%20Object%20Reference))
  ;[1 1 1] When unpossessing set animation and spawn platform
  (Class|PaperZDAnimInstance|JumptoNode (Variables|/Script/PaperZD.PaperZDAnimationComponent|GetAnimInstance (Variables|Default|GetAnimationComponent)) "UnPossessed" "Locomotion")
  (Utilities|FlowControl|Delay 1.0)
  (Game|SpawnActorfromClass "/Game/BluePrints/Cain/Cain_Possesed/BP_InvisPlatform.BP_InvisPlatform_C" (Math|Conversions|ToTransform(Vector) (Math|Transform|TransformLocation (Transformation|GetActorTransform self) "0, 0,-90.000000")) "AlwaysSpawn" self 0))

(event Game|Damage|EventAnyDamage
  (params (Damage :type Float%20%28single-precision%29) (DamageType :type Damage%20Type%20Object%20Reference) (InstigatedBy :type Controller%20Object%20Reference) (DamageCauser :type Actor%20Object%20Reference))
  ;[1 1 1] When landing on spikes create a platform and a sprite
)

(fn ConstructionScript
  (|CallParentFunction))