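; BP_Cain is the player character for a sprite-based side-scroller, with jump, dash, button interaction and a pause menu.
; Movement runs along X, with control rotation flipping the sprite to match velocity.
; Events jump animation state-machine nodes, and a movement lock engages on landing or damage.
; Damage spawns BP_Cain_Possesed in its place, destroys the character and asks GM_SideScroller to restart the player.
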(event Custom|OnDestroyed_Event
  (params (DestroyedActor :type Actor%20Object%20Reference))
  ;[1 1 1] Reset Movement lock on destroy
  (Variables|Default|SetIsMovementLocked false))

(event EventBeginPlay
  (Variables|Default|SetIsMovementLocked false))

(event EventDestroyed
  (bind _asgm_side_scroller (Utilities|Casting|CastToGM_SideScroller (Game|GetGameMode)))
  (Default|CallOnPlayerDied _asgm_side_scroller self))

(event EventTick
  (params (DeltaSeconds :type Float%20%28single-precision%29))
  (bind _returnvalue (Pawn|GetController))
  (bind _returnvalue_2 (Pawn|GetController))
  ;[1 1 1] Sprite Flipping
  (|CallParentFunction DeltaSeconds)
  (if (not (Variables|Default|GetIsMovementLocked)) ; If we can't move, force updating to last direction
    (Math|Float|CompareFloat (.X (Math|Vector|BreakVector (Variables|/Script/Engine.MovementComponent|GetVelocity (Pawn|GetMovementComponent)))) 0.0
      (:>
        ;;[0 0.4745 1] Look Right
        (Utilities|IsValid _returnvalue_2
          (:Is%20Valid
            (Pawn|SetControlRotation _returnvalue_2 (Math|Rotator|MakeRotator 0.0 0.0 0.0)))))
      (:<
        ;;[0 0.4745 1] Look Left
        (Utilities|IsValid _returnvalue
          (:Is%20Valid
            (Pawn|SetControlRotation _returnvalue (Math|Rotator|MakeRotator 0.0 0.0 1.8e+02))))))))

(event EventOnJumped
  ;[1 1 1] Triggering Jump/Fall Anim
  (Class|PaperZDAnimInstance|JumptoNode (Variables|/Script/PaperZD.PaperZDAnimationComponent|GetAnimInstance (Variables|Default|GetAnimationComponent)) "Airborne" "Locomotion"))

(event EventOnWalkingOffLedge
  (params (PreviousFloorImpactNormal :type Vector%20%28by%20ref%29 :default "0, 0, 0") (PreviousFloorContactNormal :type Vector%20%28by%20ref%29 :default "0, 0, 0") (PreviousLocation :type Vector%20%28by%20ref%29 :default "0, 0, 0") (TimeDelta :type Float%20%28single-precision%29))
  ;[1 1 1] Triggering Jump/Fall Anim
  (Class|PaperZDAnimInstance|JumptoNode (Variables|/Script/PaperZD.PaperZDAnimationComponent|GetAnimInstance (Variables|Default|GetAnimationComponent)) "Airborne" "Locomotion"))

(event EventOnLanded
  (params (Hit :type Hit%20Result%20Structure%20%28by%20ref%29))
  ;[1 1 1] Landing stopping movement
  (if (not (Variables|Default|GetIsMovementLocked))
    (Class|PaperZDAnimInstance|JumptoNode (Variables|/Script/PaperZD.PaperZDAnimationComponent|GetAnimInstance (Variables|Default|GetAnimationComponent)) "Landed" "Locomotion")
    (Components|Movement|StopMovementImmediately (Variables|Character|GetCharacterMovement))
    (Variables|Default|SetIsMovementLocked true)))

(event Game|Damage|EventAnyDamage
  (params (Damage :type Float%20%28single-precision%29) (DamageType :type Damage%20Type%20Object%20Reference) (InstigatedBy :type Controller%20Object%20Reference) (DamageCauser :type Actor%20Object%20Reference))
  ;[1 1 1] Death
  (Class|PaperZDAnimInstance|JumptoNode (Variables|/Script/PaperZD.PaperZDAnimationComponent|GetAnimInstance (Variables|Default|GetAnimationComponent)) "Damaged" "Locomotion")
  (Variables|Default|SetIsMovementLocked true)
  (Utilities|FlowControl|DoOnce false
    (:Completed
      (Game|SpawnActorfromClass "/Game/BluePrints/Cain/Cain_Possesed/BP_Cain_Possesed.BP_Cain_Possesed_C" (Transformation|GetActorTransform) "AlwaysSpawn" 0 0)
      (CallFunction|CallRestartPlayer))))

(event Input|ActionEvents|InputActionDash
  (params (Key :type Key%20Structure :default "None"))
  ;[1 1 1] Dashing
  (:Pressed
    (Variables|Default|SetRunPlayRate 1.5)
    (Variables|/Script/Engine.CharacterMovementComponent|SetMaxWalkSpeed (Variables|Character|GetCharacterMovement) 7.5e+02))
  (:Released
    (Variables|Default|SetRunPlayRate 1.0)
    (Variables|/Script/Engine.CharacterMovementComponent|SetMaxWalkSpeed (Variables|Character|GetCharacterMovement) 5e+02)))

(event Input|ActionEvents|InputActionJump
  (params (Key :type Key%20Structure :default "None"))
  ;[1 1 1] Jump Trigger
  (:Pressed
    (Character|Jump))
  (:Released
    (Character|StopJumping)))

(event Input|ActionEvents|InputActionPause
  (params (Key :type Key%20Structure :default "None"))
  (bind _returnvalue (Game|GetPlayerController 0))
  (bind _returnvalue_2 (Game|GetPlayerController 0))
  ;[1 1 1] Menu
  (:Pressed
    (Utilities|FlowControl|FlipFlop
      (:A
        (bind _returnvalue_3 (UserInterface|CreateWidget "/Game/UI/PAUSE/Pause.Pause_C"))
        (UserInterface|Viewport|AddtoViewport _returnvalue_3 0)
        (Game|SetGamePaused true)
        (Input|SetInputModeGameandUI _returnvalue 0 "DoNotLock" true)
        (Variables|/Script/Engine.PlayerController|SetbShowMouseCursor _returnvalue true))
      (:B
        (Widget|RemovefromParent _returnvalue_3)
        (Input|SetInputModeGameOnly _returnvalue_2)
        (Variables|/Script/Engine.PlayerController|SetbShowMouseCursor _returnvalue_2 false)
        (Game|SetGamePaused false)))))

(event Input|ActionEvents|InputActionInteract
  (params (Key :type Key%20Structure :default "None"))
  ;[1 1 1] Interacting with Buttons
  (:Pressed
    (bind _array_element (Utilities|Array|ForEachLoopwithBreak (Collision|GetOverlappingActors "/Game/BluePrints/Interactables/BP_Button.BP_Button_C" :!class /Script/Engine.Actor) :!label _label)
      (:LoopBody
        (if (Utilities|DoesObjectImplementInterface _array_element "/Game/BluePrints/BPI_ButtonsDoors.BPI_ButtonsDoors_C")
          (Class|BPIButtonsDoors|Interact(Message) _array_element)
          (goto _label Break))))))

(event Input|AxisEvents|InputAxisForward
  (params (AxisValue :type Float%20%28single-precision%29))
  ;[1 1 1] Movement forward
  (if (not (Variables|Default|GetIsMovementLocked))
    (Pawn|Input|AddMovementInput "1.000000, 0, 0" AxisValue false)))

(fn ConstructionScript)

(fn CallRestartPlayer
  (LocalVariables|SetControllerRef (Pawn|GetController))
  (Actor|DestroyActor)
  (bind _asgm_side_scroller (Utilities|Casting|CastToGM_SideScroller (Game|GetGameMode)))
  (Class|GameModeBase|RestartPlayer _asgm_side_scroller (LocalVariables|GetControllerRef)))