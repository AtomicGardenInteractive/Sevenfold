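; BP_Button is a one-shot Paper2D interactable that either opens a door or switches off electric floors, chosen by IsDoorController.
; Interact searches all BP_Door or BP_ElectricFloor actors for values matching ButtonValue, triggering the first matching door or every matching floor, then swaps the button sprite.
; Overlapping InteractRange clears all widgets and shows a PopUp with the button's prompt text; leaving clears all widgets again.
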(event OnComponentBeginOverlap(InteractRange)
  (params (OverlappedComponent :type Primitive%20Component%20Object%20Reference) (OtherActor :type Actor%20Object%20Reference) (OtherComp :type Primitive%20Component%20Object%20Reference) (OtherBodyIndex :type Integer) (bFromSweep :type Boolean) (SweepResult :type Hit%20Result%20Structure%20%28by%20ref%29))
  (Viewport|RemoveAllWidgets)
  (bind _returnvalue (UserInterface|CreateWidget "/Game/BluePrints/UI/PopUp.PopUp_C"))
  (Variables|/Game/BluePrints/UI/PopUp.PopUp_C|SetTEXT _returnvalue (Variables|Default|GetUITextPrompt))
  (UserInterface|Viewport|AddtoViewport _returnvalue 0)
  (Development|PrintText "Prompt Called"))

(event OnComponentEndOverlap(InteractRange)
  (params (OverlappedComponent :type Primitive%20Component%20Object%20Reference) (OtherActor :type Actor%20Object%20Reference) (OtherComp :type Primitive%20Component%20Object%20Reference) (OtherBodyIndex :type Integer))
  (Viewport|RemoveAllWidgets))

(event EventInteract
  (if (Variables|Default|GetIsDoorController)
    (if (not (Variables|Default|GetIsDoorOpen))
      (bind _outactors (Actor|GetAllActorsOfClass "/Game/BluePrints/Interactables/BP_Door.BP_Door_C"))
      (bind _array_element (Utilities|Array|ForEachLoopwithBreak _outactors :!label _label)
        (:LoopBody
          (if (== (Variables|/Game/BluePrints/Interactables/BP_Door.BP_Door_C|GetDoor%20Value _array_element) (Variables|Default|GetButton%20Value))
            (Variables|Default|SetIsDoorOpen true)
            (Default|OpenDoor _array_element)
            (Rendering|Components|Sprite|SetSprite (Variables|Default|GetPaperSprite) "/Game/Assets/Interactables/Sprite-Button-Unpressed_Sprite_0.Sprite-Button-Unpressed_Sprite_0")
            (goto _label Break)))))
    (elif (not (Variables|Default|GetIsFloorOff))
      (bind _outactors_2 (Actor|GetAllActorsOfClass "/Game/BluePrints/Interactables/BP_ElectricFloor.BP_ElectricFloor_C"))
      (bind _array_element_2 (Utilities|Array|ForEachLoopwithBreak _outactors_2)
        (:LoopBody
          (if (== (Variables|/Game/BluePrints/Interactables/BP_ElectricFloor.BP_ElectricFloor_C|GetFloorValue _array_element_2) (Variables|Default|GetButton%20Value))
            (Variables|Default|SetIsFloorOff true)
            (Default|SetFloorOff _array_element_2)
            (Rendering|Components|Sprite|SetSprite (Variables|Default|GetPaperSprite) "/Game/Assets/Interactables/Sprite-Button-Unpressed_Sprite_0.Sprite-Button-Unpressed_Sprite_0")))))))

(fn ConstructionScript)