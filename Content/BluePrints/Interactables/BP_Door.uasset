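; BP_Door is an interactable door that also serves as the exit to the next level.
; OpenDoor and CloseDoor play a sound and instantly shift the DoorClosed component up out of the way or back to its origin.
; Overlapping NextLevelTrigger as BP_Cain, but not as BP_Cain_Possesed, fades the camera out, then loads the level named by LevelName after a delay.
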(event OnComponentBeginOverlap(NextLevelTrigger)
  (params (OverlappedComponent :type Primitive%20Component%20Object%20Reference) (OtherActor :type Actor%20Object%20Reference) (OtherComp :type Primitive%20Component%20Object%20Reference) (OtherBodyIndex :type Integer) (bFromSweep :type Boolean) (SweepResult :type Hit%20Result%20Structure%20%28by%20ref%29))
  (Utilities|Casting|CastToBP_Cain_Possesed OtherActor
    (:CastFailed
      (Utilities|Casting|CastToBP_Cain OtherActor)
      (CameraFades|StartCameraFade :self (Game|GetPlayerCameraManager 0) :ToAlpha 2.0 :Duration 3.0 :bHoldWhenFinished true)
      (Utilities|FlowControl|Delay 3.0)
      (Game|OpenLevel(byName) (Variables|Default|GetLevelName)))))

(event Custom|Open%20Door
  (Audio|PlaySound2D "/Engine/EditorSounds/GamePreview/PossessPlayer.PossessPlayer" 1.0 1.0 0.0 0 0)
  (Transformation|SetRelativeLocation (Variables|Default|GetDoor%20Closed) "0, 0,1000.000000" false false))

(event Custom|Close%20Door
  (Audio|PlaySound2D "/Engine/EditorSounds/GamePreview/PossessPlayer.PossessPlayer" 1.0 1.0 0.0 0 0)
  (Transformation|SetRelativeLocation (Variables|Default|GetDoor%20Closed) "0, 0, 0" false false))

(fn ConstructionScript)