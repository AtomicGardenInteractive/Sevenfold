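; BP_ElectricFloor is an electrified floor hazard that damages the BP_Cain character when it enters the floor's box.
; On box overlap it applies a configurable damage amount to BP_Cain, but ignores BP_Cain_Possesed.
; SetFloorOn and SetFloorOff events toggle the floor's visibility, box collision and component tick, and print the new state.
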(event OnComponentBeginOverlap(Box)
  (params (OverlappedComponent :type Primitive%20Component%20Object%20Reference) (OtherActor :type Actor%20Object%20Reference) (OtherComp :type Primitive%20Component%20Object%20Reference) (OtherBodyIndex :type Integer) (bFromSweep :type Boolean) (SweepResult :type Hit%20Result%20Structure%20%28by%20ref%29))
  (Utilities|Casting|CastToBP_Cain_Possesed OtherActor
    (:CastFailed
      (bind _asbp_cain (Utilities|Casting|CastToBP_Cain OtherActor))
      (Game|Damage|ApplyDamage _asbp_cain (Variables|Default|GetDamage) 0 0))))

(event Custom|SetFloorOff
  (Rendering|SetVisibility (Variables|Default|GetElectric_Floor) false false)
  (Collision|SetCollisionEnabled (Variables|Default|GetBox) "NoCollision")
  (Components|Tick|SetComponentTickEnabled (Variables|Default|GetElectric_Floor) false)
  (Development|PrintText "Electric off"))

(event Custom|SetFloorOn
  (Rendering|SetVisibility (Variables|Default|GetElectric_Floor) true true)
  (Collision|SetCollisionEnabled (Variables|Default|GetBox) "QueryAndPhysics")
  (Components|Tick|SetComponentTickEnabled (Variables|Default|GetElectric_Floor) true)
  (Development|PrintText "Electric on"))

(event EventBeginPlay)

(event Collision|EventActorBeginOverlap
  (params (OtherActor :type Actor%20Object%20Reference)))

(event EventTick
  (params (DeltaSeconds :type Float%20%28single-precision%29)))

(fn ConstructionScript)