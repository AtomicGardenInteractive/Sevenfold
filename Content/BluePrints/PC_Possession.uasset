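; Player controller Blueprint for switching possession between pawns in a level.
; ControlNextPawn stores the given index, possesses that entry of PawnsInLevel and prints a debug message.
; The Next Pawn input only casts the controller and branches to nothing.
; Disconnected logic would gather BP_Cain_Possesed actors, then step to the next index or possess CainAlive past the list's end, but it never runs.
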(event Custom|ControlNextPawn
  (params (PawnID :type Integer))
  (bind _output_get (Variables|Default|SetControlledPawn%20ID PawnID))
  (Pawn|Possess (Utilities|Array|Get(acopy) (Variables|Default|GetPawnsInLevel) _output_get))
  (Development|PrintText "control next pawn called"))

(event EventBeginPlay)

(event EventTick
  (params (DeltaSeconds :type Float%20%28single-precision%29)))

(event Input|ActionEvents|InputActionNextPawn
  (params (Key :type Key%20Structure :default "None"))
  (:Pressed
    (Utilities|Casting|CastToPC_Possession (Game|GetPlayerController 0))
    (if (stale _bsuccess)
      _)))

(fn ConstructionScript)