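; Gnasher enemy character that patrols along the X axis and hunts Cain, ignoring his possessed variant.
; Hearing overlap turns it around, Sight overlap toggles a faster chase in its facing direction, and AttackTrigger overlap stops it, jumps to the attack animation and applies damage.
; Tick drives the chase or an idle wander built from FlipFlop, DoOnce gates and random delays that alternate direction and pauses.
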(event OnComponentBeginOverlap(Sight)
  (params (OverlappedComponent :type Primitive%20Component%20Object%20Reference) (OtherActor :type Actor%20Object%20Reference) (OtherComp :type Primitive%20Component%20Object%20Reference) (OtherBodyIndex :type Integer) (bFromSweep :type Boolean) (SweepResult :type Hit%20Result%20Structure%20%28by%20ref%29))
  ;[1 1 1] Player Spotted
  (Utilities|Casting|CastToBP_Cain_Possesed OtherActor
    (:CastFailed
      (Utilities|Casting|CastToBP_Cain OtherActor)
      (Variables|Default|SetIsHunting true))))

(event OnComponentBeginOverlap(AttackTrigger)
  (params (OverlappedComponent :type Primitive%20Component%20Object%20Reference) (OtherActor :type Actor%20Object%20Reference) (OtherComp :type Primitive%20Component%20Object%20Reference) (OtherBodyIndex :type Integer) (bFromSweep :type Boolean) (SweepResult :type Hit%20Result%20Structure%20%28by%20ref%29))
  ;[1 1 1] Attacking
  (Utilities|Casting|CastToBP_Cain_Possesed OtherActor
    (:CastFailed
      (Utilities|Casting|CastToBP_Cain OtherActor)
      (Class|PaperZDAnimInstance|JumptoNode (Variables|/Script/PaperZD.PaperZDAnimationComponent|GetAnimInstance (Variables|Default|GetAnimationComponent)) "Attack" "Gnasher_Locomotion")
      (Components|Movement|StopMovementImmediately (Variables|Character|GetCharacterMovement))
      (Variables|Default|SetIsAttacking true)
      (Game|Damage|ApplyDamage OtherActor (Variables|Default|GetDamage) 0 0))))

(event OnComponentEndOverlap(Sight)
  (params (OverlappedComponent :type Primitive%20Component%20Object%20Reference) (OtherActor :type Actor%20Object%20Reference) (OtherComp :type Primitive%20Component%20Object%20Reference) (OtherBodyIndex :type Integer))
  ;[1 1 1] Return to Walk
  (Utilities|Casting|CastToBP_Cain_Possesed OtherActor
    (:CastFailed
      (Utilities|Casting|CastToBP_Cain OtherActor)
      (Variables|Default|SetIsHunting false)
      (Variables|Default|SetGnasherRunPlayRate 1.0)
      (Variables|/Script/Engine.CharacterMovementComponent|SetMaxWalkSpeed (Variables|Character|GetCharacterMovement) 2e+02)
      (Development|PrintText "Contact Lost"))))

(event OnComponentBeginOverlap(Hearing)
  (params (OverlappedComponent :type Primitive%20Component%20Object%20Reference) (OtherActor :type Actor%20Object%20Reference) (OtherComp :type Primitive%20Component%20Object%20Reference) (OtherBodyIndex :type Integer) (bFromSweep :type Boolean) (SweepResult :type Hit%20Result%20Structure%20%28by%20ref%29))
  ;[1 1 1] Player Heard
  (Utilities|Casting|CastToBP_Cain_Possesed OtherActor
    (:CastFailed
      (Utilities|Casting|CastToBP_Cain OtherActor)
      (Utilities|FlowControl|DoOnce false :!label _label
        (:Completed
          (if (Variables|Default|GetIsRotated)
            (Variables|Default|SetIsRotated false)
            (else
              (Variables|Default|SetIsRotated true)))
          (Transformation|SetActorRotation (Math|Transform|TransformRotation (Transformation|GetActorTransform) "0,180.000000,0.000000"))
          (Development|PrintText "Heard")
          (Utilities|FlowControl|Delay 1.0)
          (goto _label Reset))))))

(event EventTick
  (params (DeltaSeconds :type Float%20%28single-precision%29))
  ;[1 1 1] Movement Idle/Hunting
  (if (Variables|Default|GetIsHunting)
    (if (Variables|Default|GetIsRotated)
      (Pawn|Input|AddMovementInput "-1.000000, 0, 0" 1.0 false)
      (else
        (Pawn|Input|AddMovementInput "1.000000, 0, 0" 1.0 false)))
    (Variables|Default|SetGnasherRunPlayRate 1.5)
    (Variables|/Script/Engine.CharacterMovementComponent|SetMaxWalkSpeed (Variables|Character|GetCharacterMovement) 6e+02)
    (elif (and (not (Variables|Default|GetIsMoving)) (not (Variables|Default|GetIsAttacking)))
      (if (stale _isa)
        (Pawn|Input|AddMovementInput "1.000000, 0, 0" 1.0 false)
        (if (Variables|Default|GetIsRotated)
          (Utilities|FlowControl|DoOnce false :!label _label
            (:Completed
              (Transformation|SetActorRotation (Math|Transform|TransformRotation (Transformation|GetActorTransform) "0,180.000000,0.000000"))
              (Variables|Default|SetIsRotated false))))
        (Utilities|FlowControl|Delay (Math|Random|RandomFloatinRange 1.0 5.0))
        (Variables|Default|SetIsMoving true)
        (Utilities|FlowControl|Delay (Math|Random|RandomFloatinRange 1.0 5.0))
        (Variables|Default|SetIsMoving false)
        (goto _label Reset)
        (else
          (Pawn|Input|AddMovementInput "-1.000000, 0,0.000000" 1.0 false)
          (if (Variables|Default|GetIsRotated)
            _
            (else
              (Utilities|FlowControl|DoOnce false :!label _label_2
                (:Completed
                  (Transformation|SetActorRotation (Math|Transform|TransformRotation (Transformation|GetActorTransform) "0,180.000000,0.000000"))
                  (Variables|Default|SetIsRotated true)))))
          (Utilities|FlowControl|Delay (Math|Random|RandomFloatinRange 1.0 5.0))
          (Variables|Default|SetIsMoving true)
          (Utilities|FlowControl|Delay (Math|Random|RandomFloatinRange 1.0 5.0))
          (Variables|Default|SetIsMoving false)
          (goto _label_2 Reset)))
      (else
        (bind _isa (Utilities|FlowControl|FlipFlop))))))

(fn ConstructionScript)